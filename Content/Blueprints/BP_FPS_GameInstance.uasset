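; FPS game instance that manages multiplayer sessions: hosting, joining, quick-join and destroying, plus storing the lobby's game type.
; Hosting creates an Advanced Sessions session, public or private, tagged with owner ID and name, then opens the chosen level as a listen server.
; Auto-join takes the first search result, or calls HostSession with no arguments when none are found.
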(event Custom|HostSession
  (params (Connections :type Integer) (Private :type Boolean) (LevelToOpen :type Name) (Session%20Name :type String))
  (bind _returnvalue (Game|GetPlayerController 0))
  ;[0.15 0.15 0.15 0.5] Create New Session
  (bind _settings (CallFunction|MakeSessionExtraSettings (Class|AdvancedSessionsLibrary|GetUniqueNetID _returnvalue) Session%20Name))
  (if Private
    (|AdvancedSession _settings _returnvalue 2 Connections false true false true true false false false true false true
      (:OnSuccess
        _))
    (else
      (|AdvancedSession _settings _returnvalue Connections 0 false true false true true false false false true false true
        (:OnSuccess
          _))))
  (Game|OpenLevel(byName) LevelToOpen true "?listen")
  (Development|PrintString "Session created"))

(event Custom|JoinSessionAuto
  ;[0.15 0.15 0.15 0.5] Create Or Join Random Session
  (bind _results (|FindSessions (Game|GetPlayerController 0) 100 false false)
    (:OnSuccess
      (if (Utilities|Array|IsNotEmpty _results)
        (Development|PrintString "Session found")
        (|JoinSession (Game|GetPlayerController 0) (Utilities|Array|Get(acopy) _results)
          (:OnSuccess
            (Development|PrintString "Session Joined")))
        (else
          (Development|PrintString "Session not found, creating one...")
          (CallFunction|HostSession 0 false "None"))))))

(event Custom|JoinSession
  (params (Session%20To%20join :type Blueprint%20Session%20Result%20Structure%20%28by%20ref%29))
  ;[0.15 0.15 0.15 0.5] Join Selected Session
  (|JoinSession (Game|GetPlayerController 0) Session%20To%20join
    (:OnSuccess
      (Development|PrintString "Session Joined"))
    (:OnFailure
      (Development|PrintString "Session not available anymore"))))

(event Custom|DestroySession
  (params (Player%20In%20Session :type Player%20Controller%20Object%20Reference))
  ;[0.15 0.15 0.15 0.5] Destroy a Session
  (|DestroySession Player%20In%20Session))

(fn RetrieveLobbyData
  (params (LobbyData :type S%20Lobby%20Data%20Structure))
  (Variables|Default|SetGameType (.gametype LobbyData)))