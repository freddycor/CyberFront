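; Lobby GameState that tracks the owner, per-player ready flags, map, game type and player limit in a single Data struct.
; Ready flags are indexed parallel to PlayerArray, and setters validate map, game type and player limit before rebuilding the struct.
; A looping timer runs a cancellable countdown, and each tick, login and logout is relayed to every BP_Lobby_PlayerController.
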(event Custom|On%20Login
  (params (Player :type Player%20Controller%20Object%20Reference))
  ;[0.15 0.15 0.15 0.5] Login / Logout
  (Utilities|Array|Add (.playerstatuses (Variables|Default|GetData)) false)
  (for _array_element (Variables|Default|GetPlayerArray)
    (bind _asbp_lobby_player_controller (Utilities|Casting|CastToBP_Lobby_PlayerController (Game|GetPlayerController _array_element)))
    (Default|OnLogin _asbp_lobby_player_controller Player)))

(event Custom|Decrement%20Countdown
  (bind _countdowntime (Variables|Default|GetCountdownTime))
  ;[0.15 0.15 0.15 0.5] Countdown
  (Math|Integer|DecrementInt _countdowntime
    (:%20%20
      (if (<= _countdowntime 0)
        (Utilities|Time|ClearandInvalidateTimerbyHandle (Variables|Default|GetCountdownHandler))
        (Variables|Default|SetInCountdown false))
      (for _array_element (Variables|Default|GetPlayerArray)
        (bind _asbp_lobby_player_controller (Utilities|Casting|CastToBP_Lobby_PlayerController (Game|GetPlayerController _array_element)))
        (Default|OnDecrementedCountdown _asbp_lobby_player_controller)))))

(event Custom|Cancel%20Countdown
  ;[0.15 0.15 0.15 0.5] Countdown
  (Utilities|Time|ClearandInvalidateTimerbyHandle (Variables|Default|GetCountdownHandler))
  (Variables|Default|SetInCountdown false)
  (Variables|Default|SetCountdownTime 10))

(event Custom|Start%20Countdown
  ;[0.15 0.15 0.15 0.5] Countdown
  (Variables|Default|SetCountdownTime 10)
  (Variables|Default|SetInCountdown true)
  (bind _returnvalue (Utilities|Time|SetTimerbyFunctionName 0 "Decrement Countdown" 1.0 true))
  (Variables|Default|SetCountdownHandler _returnvalue))

(event Custom|On%20Logout
  (params (Player :type Controller%20Object%20Reference))
  (bind _playerstate (Variables|/Script/Engine.Controller|GetPlayerState Player))
  (bind _index (CallFunction|GetPlayerIndex _playerstate))
  ;[0.15 0.15 0.15 0.5] Login / Logout
  (if (>= _index 0)
    (Utilities|Array|RemoveIndex (.playerstatuses (Variables|Default|GetData)) _index)
    (for _array_element (Variables|Default|GetPlayerArray)
      (bind _asbp_lobby_player_controller (Utilities|Casting|CastToBP_Lobby_PlayerController (Game|GetPlayerController _array_element)))
      (Default|OnLogout _asbp_lobby_player_controller Player))))

(event EventBeginPlay
  (Utilities|Array|AddUnique (.playerstatuses (Variables|Default|GetData)) false)
  (Variables|Default|SetData (Utilities|Struct|MakeS_LobbyData (Game|GetPlayerState 0) (.maxplayers (Variables|Default|GetData)) (.playerstatuses (Variables|Default|GetData)) (.map (Variables|Default|GetData)) (.gametype (Variables|Default|GetData)))))

(fn ConstructionScript)

(fn GetPlayerIndex
  (params (Player :type Player%20State%20Object%20Reference))
  (for (_array_element _array_index) (Variables|Default|GetPlayerArray)
    (if (== Player _array_element)
      (return _array_index)))
  (return -1))

(fn AreAllReady
  (for _array_element (Variables|Default|GetPlayerArray)
    (if (not (CallFunction|IsReady _array_element))
      (return false)))
  (return true))

(fn IsReady
  (params (Player :type Player%20State%20Object%20Reference))
  (bind _index (CallFunction|GetPlayerIndex Player))
  (if (< _index 0)
    (return false)
    (else
      (return (Utilities|Array|Get(acopy) (.playerstatuses (Variables|Default|GetData)) _index)))))

(fn ToggleReady
  (params (Player%20State :type Player%20State%20Object%20Reference))
  (bind _index (CallFunction|GetPlayerIndex Player%20State))
  (if (< _index 0)
    (return false)
    (else
      (Utilities|Array|SetArrayElem (.playerstatuses (Variables|Default|GetData)) _index (not (CallFunction|IsReady Player%20State))))))

(fn SetMap
  (params (Internal%20Map%20Name :type Name))
  (if (CallFunction|IsValidMapName Internal%20Map%20Name)
    (Variables|Default|SetData (Utilities|Struct|MakeS_LobbyData (.owner (Variables|Default|GetData)) (.maxplayers (Variables|Default|GetData)) (.playerstatuses (Variables|Default|GetData)) Internal%20Map%20Name (.gametype (Variables|Default|GetData))))))

(fn IsOwner
  (params (Player%20State :type Player%20State%20Object%20Reference))
  (return (== Player%20State (.owner (Variables|Default|GetData)))))

(fn SetMaxPlayers
  (params (Max%20Players :type Integer))
  (bind _output_get (LocalVariables|SetTo%20Set Max%20Players))
  (if (and (> _output_get (Utilities|Array|Length (Variables|Default|GetPlayerArray))) (> _output_get 1))
    (Variables|Default|SetData (Utilities|Struct|MakeS_LobbyData (.owner (Variables|Default|GetData)) _output_get (.playerstatuses (Variables|Default|GetData)) (.map (Variables|Default|GetData)) (.gametype (Variables|Default|GetData))))))

(fn SetGameType
  (params (Game%20Type :type GameType%20Enum :default "NewEnumerator0"))
  (bind _data (CallFunction|GetMapData (.map (Variables|Default|GetData))))
  (if (Utilities|Set|Contains (.supportedgametypes _data) Game%20Type)
    (Variables|Default|SetData (Utilities|Struct|MakeS_LobbyData (.owner (Variables|Default|GetData)) (.maxplayers (Variables|Default|GetData)) (.playerstatuses (Variables|Default|GetData)) (.map (Variables|Default|GetData)) Game%20Type))))