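; Base weapon Blueprint that handles barrel heat distortion, skin overlays and stat previews.
; Firing adds clamped heat and a looping 0.1-second timer cools it, both feeding the heat amount into a Niagara distortion effect.
; It also builds preview stats with Italian display names, flagging reload time and recoil as reversed, and applies skins as skeletal mesh overlay materials.
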(event Custom|On%20Fire
  (bind _output_get (Variables|HeatDistortion|SetHT_CurrentHeat (Math|Float|Clamp(Float) (+ (Variables|HeatDistortion|GetHT_CurrentHeat) (Variables|HeatDistortion|GetHT_HeatRate)))))
  (Niagara|SetNiagaraVariable(Float) (Variables|Default|GetNS_HeatDistortion) "HeatAmount" _output_get))

(event EventBeginPlay
  ;[0.15 0.15 0.15 0.5] Heat Distortion
  (Class|NiagaraComponent|SetVariableVec2 (Variables|Default|GetNS_HeatDistortion) "SpriteSizeRange" (Variables|HeatDistortion|GetHT_SizeRange))
  ;[0.15 0.15 0.15 0.5] Cooling
  (Utilities|Time|SetTimerbyFunctionName 0 "coolingFunc" 0.1 true))

(fn ConstructionScript)

(fn CoolingFunc
  (bind _output_get (Variables|HeatDistortion|SetHT_CurrentHeat (Math|Float|Clamp(Float) (- (Variables|HeatDistortion|GetHT_CurrentHeat) (* (Variables|HeatDistortion|GetHT_CoolingRate) 0.1)))))
  (Niagara|SetNiagaraVariable(Float) (Variables|Default|GetNS_HeatDistortion) "HeatAmount" _output_get))

(fn MakePreviewStats
  (bind _stats (Variables|Default|GetStats))
  (return (Utilities|Struct|MakeS_WeaponPreview_Stats (Variables|Default|GetType) (Variables|Default|GetName) (Utilities|Array|MakeArray (Utilities|Struct|MakeS_WeaponPreview_Stat "Damage" "Danno" (.damage _stats) 1e+02) (Utilities|Struct|MakeS_WeaponPreview_Stat "FireRate" "Rateo di Fuoco" (.firerate _stats) 1e+03) (Utilities|Struct|MakeS_WeaponPreview_Stat "ReloadTime" "Tempo di Ricarica" (.reloadtime _stats) 1e+01 true) (Utilities|Struct|MakeS_WeaponPreview_Stat "Recoil" "Rinculo" (.recoilforce _stats) 1.0 true)))))

(fn SetSkin
  (params (NewOverlayMaterial :type Material%20Interface%20Object%20Reference))
  (Rendering|Material|SetOverlayMaterial (Variables|Default|GetSkeletalMesh) NewOverlayMaterial :!class /Script/Engine.MeshComponent))