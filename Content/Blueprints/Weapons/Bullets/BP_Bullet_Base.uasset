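; Base bullet actor for FPS weapons that handles impacts, player damage and near-miss whiz sounds.
; On hit it fires a radial impulse, destroys itself and plays impact effects.
; For player hits, the server checks GameHandler, applies the shooter's weapon damage, shows a hit marker, counts the hit and traces onward to spawn blood.
; WhizCollider end-overlap plays a delayed whip sound for nearby local players unless flagged IsHit.
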(event OnComponentEndOverlap(WhizCollider)
  (params (OverlappedComponent :type Primitive%20Component%20Object%20Reference) (OtherActor :type Actor%20Object%20Reference) (OtherComp :type Primitive%20Component%20Object%20Reference) (OtherBodyIndex :type Integer))
  ;[0.15 0.15 0.15 0.5] Whiz Effect
  ;;[0.15 0.15 0.15 0.5] If Player
  (bind _asbp_fps_character (Utilities|Casting|CastToBP_FPS_Character OtherActor))
  (if (Math|Boolean|ANDBoolean (Pawn|IsLocallyControlled _asbp_fps_character) (!= _asbp_fps_character (Variables|Actor|GetInstigator)) (< (Transformation|GetHorizontalDistanceTo _asbp_fps_character self) 5e+02))
    (Utilities|FlowControl|Delay 0.2)
    (if (not (Variables|/Game/Blueprints/Match/Player/BP_FPS_Character.BP_FPS_Character_C|GetisHit _asbp_fps_character))
      (Audio|PlaySoundatLocation "/Game/Audio/Sounds/Rifle_Whip01.Rifle_Whip01" (Transformation|GetWorldLocation (Variables|Default|GetBullet)) "0, 0, 0" 1.0 1.0 0.0 0 0 0 0))))

(event OnComponentHit(Box)
  (params (HitComponent :type Primitive%20Component%20Object%20Reference) (OtherActor :type Actor%20Object%20Reference) (OtherComp :type Primitive%20Component%20Object%20Reference) (NormalImpulse :type Vector :default "0, 0, 0") (Hit :type Hit%20Result%20Structure%20%28by%20ref%29))
  (bind _location (Collision|BreakHitResult Hit))
  (bind _fps_character (CallFunction|GetShooter))
  (bind _fps_character_2 (CallFunction|GetShooter))
  (bind _player_state (Default|GetPlayerState _fps_character_2))
  (bind _weapon (Default|GetWeaponData _fps_character))
  (bind _stats (Variables|/Game/Blueprints/Weapons/BP_Weapon_Base.BP_Weapon_Base_C|GetStats _weapon))
  (Class|RadialForceComponent|FireImpulse (Variables|Default|GetRadialForce))
  (Actor|DestroyActor)
  (CallFunction|PlayImpactSound OtherActor _location)
  (CallFunction|SpawnEmitter _location)
  ;[0.15 0.15 0.15 0.5] If Player
  (bind _asbp_fps_character (Utilities|Casting|CastToBP_FPS_Character OtherActor))
  ;[0.15 0.15 0.15 0.5] Player Damage Handler
  (Networking|SwitchHasAuthority
    (:Authority
      ;;[0.15 0.15 0.15 0.5] Check if can damage (same team)
      (if (Default|ShouldDamage (Variables|/Game/Blueprints/Match/BP_FPS_GameMode.BP_FPS_GameMode_C|GetGameHandler (CallFunction|GetGameMode)) _asbp_fps_character (CallFunction|GetShooter))
        ;;[0.15 0.15 0.15 0.5] Hit Marker
        (Default|HitMarker (CallFunction|GetShooter) (<= (Variables|/Game/Blueprints/Match/Player/BP_FPS_Character.BP_FPS_Character_C|Gethealth _asbp_fps_character) (.damage _stats)))
        ;;[0.15 0.15 0.15 0.5] Apply Damage to hit Player
        (Game|Damage|ApplyDamage _asbp_fps_character (.damage _stats) 0 _fps_character)
        (Utilities|FlowControl|Sequence
          (:then_1
            ;[0.15 0.15 0.15 0.5] Add Hits to Damager
            (Variables|/Game/Blueprints/Match/Player/BP_FPS_PlayerState.BP_FPS_PlayerState_C|SethitsDone _player_state (+ (Variables|/Game/Blueprints/Match/Player/BP_FPS_PlayerState.BP_FPS_PlayerState_C|GethitsDone _player_state) 1)))
          (:then_2
            ;[0.15 0.15 0.15 0.5] Whiz Fix
            (Variables|/Game/Blueprints/Match/Player/BP_FPS_Character.BP_FPS_Character_C|SetisHit _asbp_fps_character true)
            (Utilities|FlowControl|Delay 0.4)
            (Variables|/Game/Blueprints/Match/Player/BP_FPS_Character.BP_FPS_Character_C|SetisHit _asbp_fps_character false))
          (:then_3
            ;[0.15 0.15 0.15 0.5] Blood Spawning
            (bind (_outhit _returnvalue) (Collision|LineTraceByChannel _location (+ _location (* (Transformation|GetActorForwardVector) 3e+02)) "TraceTypeQuery1" false (Utilities|Array|MakeArray _asbp_fps_character) "None"))
            (if _returnvalue
              (Game|SpawnActorfromClass "/Game/FX/BP_Blood.BP_Blood_C" (Math|Transform|MakeTransform (.Location (Collision|BreakHitResult _outhit)) (Math|Conversions|RotationFromXVector (.Normal (Collision|BreakHitResult _outhit)))) "Undefined" "MultiplyWithRoot" 0 0))))))))

(event EventBeginPlay
  (bind _instigator (Variables|Actor|GetInstigator))
  (Collision|IgnoreActorwhenMoving (Variables|Default|GetBox) _instigator true)
  (bind _asbp_fps_character (Utilities|Casting|CastToBP_FPS_Character _instigator))
  (Collision|IgnoreActorwhenMoving (Variables|/Script/Engine.Character|GetCapsuleComponent _asbp_fps_character) self true)
  (Utilities|FlowControl|Delay 2.0))

(fn ConstructionScript)

(fn GetShooter
  (bind _asbp_fps_character (Utilities|Casting|CastToBP_FPS_Character (Variables|Actor|GetInstigator)))
  (return _asbp_fps_character))

(fn PlayImpactSound
  (params (Hit%20Actor :type Actor%20Object%20Reference) (Location :type Vector))
  (bind _sounds (Variables|Default|GetSounds))
  (Utilities|Casting|CastToBP_FPS_Character Hit%20Actor
    (:then
      (LocalVariables|SetToPlay (.impactbody _sounds)))
    (:CastFailed
      (LocalVariables|SetToPlay (.impactsurface _sounds))))
  (Utilities|IsValid (LocalVariables|GetToPlay)
    (:Is%20Valid
      (Audio|PlaySoundatLocation (LocalVariables|GetToPlay) Location "0, 0, 0" 1.0 1.0 0.0 0 0 0 0))))

(fn SpawnEmitter
  (params (Location :type Vector))
  (bind _impactemitter (Variables|Default|GetImpactEmitter))
  (Utilities|IsValid _impactemitter
    (:Is%20Valid
      (Effects|SpawnEmitteratLocation _impactemitter Location))))