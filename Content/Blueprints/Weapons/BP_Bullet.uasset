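; BP_Bullet is a short-lived FPS projectile that ignores its shooter and destroys itself on impact or after two seconds.
; Hits fire a radial impulse plus body or surface sound and an emitter.
; For player victims, the authority checks team rules through the GameHandler, applies the shooter's current weapon damage, plays a hit marker and counts the hit.
; A separate collider plays a whiz sound for nearby locally controlled non-shooters.
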(event OnComponentBeginOverlap(WhizCollider)
  (params (OverlappedComponent :type Primitive%20Component%20Object%20Reference) (OtherActor :type Actor%20Object%20Reference) (OtherComp :type Primitive%20Component%20Object%20Reference) (OtherBodyIndex :type Integer) (bFromSweep :type Boolean) (SweepResult :type Hit%20Result%20Structure%20%28by%20ref%29))
  ;[0.15 0.15 0.15 0.5] Whiz Effect
  ;;[0.15 0.15 0.15 0.5] If Player
  (bind _asbp_fps_character (Utilities|Casting|CastToBP_FPS_Character OtherActor))
  (if (and (Pawn|IsLocallyControlled _asbp_fps_character) (!= _asbp_fps_character (Variables|Actor|GetInstigator)))
    (Audio|PlaySoundatLocation "/Game/Audio/Sounds/Rifle_Whip01.Rifle_Whip01" (Transformation|GetWorldLocation (Variables|Default|GetBullet)) "0, 0, 0" 1.0 1.0 0.0 0 0 0 0)))

(event OnComponentHit(Box)
  (params (HitComponent :type Primitive%20Component%20Object%20Reference) (OtherActor :type Actor%20Object%20Reference) (OtherComp :type Primitive%20Component%20Object%20Reference) (NormalImpulse :type Vector :default "0, 0, 0") (Hit :type Hit%20Result%20Structure%20%28by%20ref%29))
  (bind _location (Collision|BreakHitResult Hit))
  (bind _fps_character (CallFunction|GetShooter))
  (bind _fps_character_2 (CallFunction|GetShooter))
  (bind _player_state (Default|GetPlayerState _fps_character_2))
  (Class|RadialForceComponent|FireImpulse (Variables|Default|GetRadialForce))
  (Actor|DestroyActor)
  (CallFunction|PlayImpactSound OtherActor _location)
  (CallFunction|SpawnEmitter _location)
  ;[0.15 0.15 0.15 0.5] If Player
  (bind _asbp_fps_character (Utilities|Casting|CastToBP_FPS_Character OtherActor))
  ;[0.15 0.15 0.15 0.5] Player Damage Handler
  (Networking|SwitchHasAuthority
    (:Authority
      ;;[0.15 0.15 0.15 0.5] Check if can damage (same team)
      (if (Default|ShouldDamage (Variables|/Game/Blueprints/Match/BP_FPS_GameMode.BP_FPS_GameMode_C|GetGameHandler (CallFunction|GetGameMode)) _asbp_fps_character (CallFunction|GetShooter))
        ;;[0.15 0.15 0.15 0.5] Apply Damage to hit Player
        (Game|Damage|ApplyDamage _asbp_fps_character (.Damage (Utilities|Struct|BreakWeapon_Stats (.stats (.Item (Default|GetCurrentItem _fps_character))))) 0 _fps_character)
        (Utilities|FlowControl|Sequence
          (:then_0
            ;;[0.15 0.15 0.15 0.5] Hit Marker
            (Default|PlaySoundfromServer (CallFunction|GetShooter) "/Game/Audio/Sounds/HitMarker.HitMarker" "0, 0, 0" 0.1))
          (:then_1
            ;;[0.15 0.15 0.15 0.5] Add Hits to Damager
            (Variables|/Game/Blueprints/Match/Player/BP_FPS_PlayerState.BP_FPS_PlayerState_C|SethitsDone _player_state (+ (Variables|/Game/Blueprints/Match/Player/BP_FPS_PlayerState.BP_FPS_PlayerState_C|GethitsDone _player_state) 1))))))))

(event EventBeginPlay
  (bind _instigator (Variables|Actor|GetInstigator))
  (Collision|IgnoreActorwhenMoving (Variables|Default|GetBox) _instigator true)
  (bind _asbp_fps_character (Utilities|Casting|CastToBP_FPS_Character _instigator))
  (Collision|IgnoreActorwhenMoving (Variables|/Script/Engine.Character|GetCapsuleComponent _asbp_fps_character) self true)
  (Utilities|FlowControl|Delay 2.0)
  (Actor|DestroyActor))

(fn ConstructionScript)

(fn GetShooter
  (bind _asbp_fps_character (Utilities|Casting|CastToBP_FPS_Character (Variables|Actor|GetInstigator)))
  (return _asbp_fps_character))

(fn PlayImpactSound
  (params (Hit%20Actor :type Actor%20Object%20Reference) (Location :type Vector))
  (bind _weaponusedsounds (Variables|Default|GetWeaponUsedSounds))
  (bind (_impactsurface _impactbody) (Utilities|Struct|BreakBulletSounds (.bullet _weaponusedsounds)))
  (Utilities|Casting|CastToBP_FPS_Character Hit%20Actor
    (:then
      (LocalVariables|SetToPlay _impactbody))
    (:CastFailed
      (LocalVariables|SetToPlay _impactsurface)))
  (Utilities|IsValid (LocalVariables|GetToPlay)
    (:Is%20Valid
      (Audio|PlaySoundatLocation (LocalVariables|GetToPlay) Location "0, 0, 0" 1.0 1.0 0.0 0 0 0 0))))

(fn SpawnEmitter
  (params (Location :type Vector))
  (bind _emitter (Variables|Default|GetEmitter))
  (Utilities|IsValid _emitter
    (:Is%20Valid
      (Effects|SpawnEmitteratLocation _emitter Location))))