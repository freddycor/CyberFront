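; Blueprint function library for building and reading online session extra settings that store a session's name and owner.
; It writes the owner's unique net ID as a string alongside the name, and the getters return an empty string when a key is missing or wrongly typed.
; Ownership checks compare that stored string to a player's net ID, with a Player Controller overload that returns false for invalid controllers.
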(fn GetSessionName
  (params (Extra%20Settings :type Array%20of%20Session%20Property%20Key%20Pair%20Structures))
  (bind _settingvalue (Class|AdvancedSessionsLibrary|GetSessionPropertyString Extra%20Settings "Name")
    (:Found
      (return _settingvalue))
    (:NotFound
      _)
    (:WrongType
      _))
  (return ""))

(fn GetSessionOwner
  (params (Extra%20Settings :type Array%20of%20Session%20Property%20Key%20Pair%20Structures))
  (bind _settingvalue (Class|AdvancedSessionsLibrary|GetSessionPropertyString Extra%20Settings "Owner")
    (:Found
      (return _settingvalue))
    (:NotFound
      _)
    (:WrongType
      _))
  (return ""))

(fn IsSessionOwner(NetId)
  (params (Extra%20Settings :type Array%20of%20Session%20Property%20Key%20Pair%20Structures) (Player%20Net%20Id :type BP%20Unique%20Net%20Id%20Structure))
  (return (Utilities|Enum|Equal(Enum) (CallFunction|GetSessionOwner Extra%20Settings) (Class|AdvancedSessionsLibrary|UniqueNetIdtoString Player%20Net%20Id))))

(fn IsSessionOwner(PlayerController)
  (params (Extra%20Settings :type Array%20of%20Session%20Property%20Key%20Pair%20Structures) (Player%20Controller :type Player%20Controller%20Object%20Reference))
  (Utilities|IsValid Player%20Controller
    (:Is%20Valid
      (return (CallFunction|IsSessionOwner(NetId) Extra%20Settings (Class|AdvancedSessionsLibrary|GetUniqueNetID Player%20Controller))))
    (:Is%20Not%20Valid
      (return false))))

(fn MakeSessionExtraSettings
  (params (Owner :type BP%20Unique%20Net%20Id%20Structure) (Name :type String))
  (return (Utilities|Array|MakeArray (Class|AdvancedSessionsLibrary|MakeLiteralSessionPropertyString "Owner" (Class|AdvancedSessionsLibrary|UniqueNetIdtoString Owner)) (Class|AdvancedSessionsLibrary|MakeLiteralSessionPropertyString "Name" Name))))