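; Player state for an FPS match that tracks the player's kills, deaths and kill streak.
; On begin play it binds to the game state's kill event, with HandleKill as the evident handler.
; On the authority, a kill by this player raises kills and streak, while a death raises deaths and resets streak.
; Kill changes fire the game state's score change event directly on the server and through OnRep on clients.
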(event EventBeginPlay
  (EventDispatchers|BindEventtoKillEvent (CallFunction|GetGameState) (EventDispatchers|CreateEvent :!event HandleKill)))

(event EventTick
  (params (DeltaSeconds :type Float%20%28single-precision%29)))

(fn ConstructionScript)

(fn OnRepKills
  (Default|CallScoreChangeEvent (CallFunction|GetGameState)))

(fn HandleKill
  (params (Victim :type BP%20FPS%20Character%20Object%20Reference) (Killer :type BP%20FPS%20Character%20Object%20Reference) (VictimPlayerState :type BP%20FPS%20Player%20State%20Object%20Reference) (KillerPlayerState :type BP%20FPS%20Player%20State%20Object%20Reference))
  (Networking|SwitchHasAuthority
    (:Authority
      (Utilities|FlowControl|Sequence
        (:then_0
          ;[0.15 0.15 0.15 0.5] Handle Killer Stats
          (if (== KillerPlayerState self)
            (Math|Integer|IncrementInt (Variables|stats|Getkills)
              (:%20%20
                (Math|Integer|IncrementInt (Variables|stats|Getstreak)
                  (:%20%20
                    (Default|CallScoreChangeEvent (CallFunction|GetGameState))))))))
        (:then_1
          ;[0.15 0.15 0.15 0.5] Handle Victim Stats
          (if (== VictimPlayerState self)
            (Math|Integer|IncrementInt (Variables|stats|Getdeaths)
              (:%20%20
                (Variables|stats|Setstreak 0)))))))))