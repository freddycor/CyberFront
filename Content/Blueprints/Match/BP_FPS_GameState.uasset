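; FPS match game state that maintains a leaderboard of player states ranked by kills, highest first.
; On BeginPlay it binds a handler to the score change event, which handlePlayerJoin also fires when called.
; CalculateLeaderboard sorts all player states with a comparator delegate in reverse, casts them to BP_FPS_PlayerState and stores the result in SortedPlayers.
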(event Custom|handlePlayerJoin
  (Default|CallScoreChangeEvent))

(event EventBeginPlay
  (EventDispatchers|BindEventtoScoreChangeEvent (EventDispatchers|CreateEvent :!event CalculateLeaderboard)))

(event EventTick
  (params (DeltaSeconds :type Float%20%28single-precision%29)))

(fn ConstructionScript)

(fn CalculateLeaderboard
  (bind _sortedplayerslocal (LocalVariables|GetsortedPlayersLocal))
  (for _array_element (Class|LowEntryExtendedStandardLibrary|SortObjectArray (CallFunction|GetAllPlayerStates) (EventDispatchers|CreateEvent :!event ComparatorPlayers) true)
    (bind _asbp_fps_player_state (Utilities|Casting|CastToBP_FPS_PlayerState _array_element))
    (Utilities|Array|Add _sortedplayerslocal _asbp_fps_player_state))
  (Variables|Default|SetsortedPlayers _sortedplayerslocal))

(fn ComparatorPlayers
  (params (ObjectA :type Object%20Object%20Reference) (ObjectB :type Object%20Object%20Reference))
  (bind _asbp_fps_player_state (Utilities|Casting|CastToBP_FPS_PlayerState ObjectA))
  (bind _asbp_fps_player_state_2 (Utilities|Casting|CastToBP_FPS_PlayerState ObjectB))
  (return (< (Variables|/Game/Blueprints/Match/Player/BP_FPS_PlayerState.BP_FPS_PlayerState_C|Getkills _asbp_fps_player_state) (Variables|/Game/Blueprints/Match/Player/BP_FPS_PlayerState.BP_FPS_PlayerState_C|Getkills _asbp_fps_player_state_2))))