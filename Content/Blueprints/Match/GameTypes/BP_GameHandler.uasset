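; BP_GameHandler defines match rules with default behavior for spawning, damage, teams, kills, win checks and winner lookup.
; Respawns pick a random BP_SpawnPoint whose GameType contains the game state's current type.
; Start calls an empty AssignTeams and sets PointsToWin, while IsFinished separately checks player kills against a hardcoded threshold.
; Damage is always allowed, OnKill does nothing and GetWinner returns "None".
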(event EventBeginPlay)

(event Collision|EventActorBeginOverlap
  (params (OtherActor :type Actor%20Object%20Reference)))

(event EventTick
  (params (DeltaSeconds :type Float%20%28single-precision%29)))

(fn ConstructionScript)

(fn GetRespawnLocation
  (params (Controller :type Controller%20Object%20Reference))
  (return (Transformation|GetActorTransform (.OutItem (Utilities|Array|Random (CallFunction|GetModeSpawnPoints))))))

(fn IsFinished
  (bind _outactors (Actor|GetAllActorsOfClass "/Game/Blueprints/Match/Player/BP_FPS_PlayerState.BP_FPS_PlayerState_C"))
  (for _array_element _outactors
    (if (>= (Variables|/Game/Blueprints/Match/Player/BP_FPS_PlayerState.BP_FPS_PlayerState_C|Getkills _array_element) 2)
      (return true)))
  (return false))

(fn ShouldDamage
  (params (Victim :type BP%20FPS%20Character%20Object%20Reference) (Damager :type BP%20FPS%20Character%20Object%20Reference))
  (return true))

(fn AssignTeams)

(fn GetModeSpawnPoints
  (bind _possiblespawnsarray (LocalVariables|GetPossibleSpawnsArray))
  (bind _outactors (Actor|GetAllActorsOfClass "/Game/Blueprints/Match/BP_SpawnPoint.BP_SpawnPoint_C"))
  (for _array_element _outactors
    (if (Utilities|Array|ContainsItem (Variables|/Game/Blueprints/Match/BP_SpawnPoint.BP_SpawnPoint_C|GetGameType _array_element) (Variables|/Game/Blueprints/Match/BP_FPS_GameState.BP_FPS_GameState_C|GetGameType (CallFunction|GetGameState)))
      (Utilities|Array|Add _possiblespawnsarray _array_element)))
  (return _possiblespawnsarray))

(fn OnKill
  (params (Victim :type BP%20FPS%20Character%20Object%20Reference) (Damager :type BP%20FPS%20Character%20Object%20Reference))
  (return))

(fn HandleStart
  (CallFunction|AssignTeams)
  (Variables|/Game/Blueprints/Match/BP_FPS_GameState.BP_FPS_GameState_C|SetpointsToWin (CallFunction|GetGameState) 2))

(fn GetWinner
  (return "None"))