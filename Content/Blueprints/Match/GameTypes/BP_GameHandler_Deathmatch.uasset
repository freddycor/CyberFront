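; BP_GameHandler_Deathmatch is a match handler implementing two-team deathmatch rules, where kills score points for the killer's team.
; It assigns teams by alternating player index, blocks friendly fire, and respawns players at the first spawn point matching their team.
; Team points live in the game state; the match finishes when either team reaches the target set at start, and the leader is named BLU or ROSSO.
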(event EventBeginPlay
  (|CallParentFunction))

(event Collision|EventActorBeginOverlap
  (params (OtherActor :type Actor%20Object%20Reference))
  (|CallParentFunction OtherActor) ; This node is disabled and will not be called.\nDrag off pins to build functionality.
)

(event EventTick
  (params (DeltaSeconds :type Float%20%28single-precision%29))
  (|CallParentFunction DeltaSeconds) ; This node is disabled and will not be called.\nDrag off pins to build functionality.
)

(fn ConstructionScript
  (|CallParentFunction))

(fn ShouldDamage
  (params (Victim :type BP%20FPS%20Character%20Object%20Reference) (Damager :type BP%20FPS%20Character%20Object%20Reference))
  (return (!= (Variables|/Game/Blueprints/Match/Player/BP_FPS_PlayerState.BP_FPS_PlayerState_C|GetTeam (Default|GetPlayerState Damager)) (Variables|/Game/Blueprints/Match/Player/BP_FPS_PlayerState.BP_FPS_PlayerState_C|GetTeam (Default|GetPlayerState Victim)))))

(fn AssignTeams
  (for (_array_element _array_index) (CallFunction|GetAllPlayerStates)
    (Variables|/Game/Blueprints/Match/Player/BP_FPS_PlayerState.BP_FPS_PlayerState_C|SetTeam _array_element (Math|Integer|SelectInt 0 1 (== (Math|Integer|%(Integer) _array_index 2) 0)))))

(fn GetRespawnLocation
  (params (Controller :type Controller%20Object%20Reference))
  (bind _possiblespawnpoints (LocalVariables|GetPossibleSpawnPoints))
  (bind _asbp_fps_player_state (Utilities|Casting|CastToBP_FPS_PlayerState (Variables|/Script/Engine.Controller|GetPlayerState Controller)))
  (for _array_element (CallFunction|GetModeSpawnPoints)
    (if (== (Variables|/Game/Blueprints/Match/Player/BP_FPS_PlayerState.BP_FPS_PlayerState_C|GetTeam _asbp_fps_player_state) (Variables|/Game/Blueprints/Match/BP_SpawnPoint.BP_SpawnPoint_C|GetTeam _array_element))
      (Utilities|Array|Add _possiblespawnpoints _array_element)))
  (return (Transformation|GetActorTransform (Utilities|Array|Get(acopy) _possiblespawnpoints))))

(fn OnKill
  (params (Victim :type BP%20FPS%20Character%20Object%20Reference) (Damager :type BP%20FPS%20Character%20Object%20Reference))
  (bind _player_state (Default|GetPlayerState Damager))
  (bind _fps_gamestate (CallFunction|GetGameState))
  (bind _points (Variables|/Game/Blueprints/Match/BP_FPS_GameState.BP_FPS_GameState_C|Getpoints _fps_gamestate))
  (bind _team (Variables|/Game/Blueprints/Match/Player/BP_FPS_PlayerState.BP_FPS_PlayerState_C|GetTeam _player_state))
  (Utilities|Array|SetArrayElem _points _team (+ (Utilities|Array|Get(acopy) _points _team) 1) true))

(fn HandleStart
  (|CallParentFunction)
  (Variables|/Game/Blueprints/Match/BP_FPS_GameState.BP_FPS_GameState_C|SetpointsToWin (CallFunction|GetGameState) 5))

(fn IsFinished
  (bind _fps_gamestate (CallFunction|GetGameState))
  (for _array_element (Variables|/Game/Blueprints/Match/BP_FPS_GameState.BP_FPS_GameState_C|Getpoints _fps_gamestate)
    (if (>= _array_element (Variables|/Game/Blueprints/Match/BP_FPS_GameState.BP_FPS_GameState_C|GetpointsToWin _fps_gamestate))
      (return true)))
  (return false))

(fn GetWinner
  (for (_array_element _array_index) (Variables|/Game/Blueprints/Match/BP_FPS_GameState.BP_FPS_GameState_C|Getpoints (CallFunction|GetGameState))
    (if (> _array_element (LocalVariables|GetWinnerPoints))
      (LocalVariables|SetWinners _array_index)
      (LocalVariables|SetWinnerPoints _array_element)))
  (return (Utilities|Select :Index (LocalVariables|GetWinners) :Option%200 "BLU" :Option%201 "ROSSO")))